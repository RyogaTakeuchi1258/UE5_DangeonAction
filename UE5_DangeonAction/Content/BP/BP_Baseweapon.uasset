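; BP_Baseweapon is a weapon Blueprint that damages actors its collision component overlaps, excluding its owner.
; WeaponActive and WeaponDeactive switch that collision on and off by setting an overlap-all profile or disabling collision.
; Each overlap applies the Damage value through a DoOnce that resets after a short delay, throttling hits across all targets rather than per actor.
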(event `self.weponcollision.OnComponentBeginOverlap`
  (params (OverlappedComponent :type "PrimitiveComponent Object Reference") (OtherActor :type "Actor Object Reference") (OtherComp :type "PrimitiveComponent Object Reference") (OtherBodyIndex :type Integer) (bFromSweep :type Boolean) (SweepResult :type "HitResult Structure (by ref)"))
  (if (!= OtherActor (`self.GetOwner`))
    (`/Engine/EditorBlueprintResources/StandardMacros.DoOnce` false :!label _label
      (:`Completed`
        (`GameplayStatics.ApplyDamage` OtherActor (`self.damage`))
        (`KismetSystemLibrary.Delay` 0.2)
        (goto _label :!via `Reset`)))))

(event `WeaponActive`
  (`PrimitiveComponent.SetCollisionProfileName` (`self.weponcollision`) "OverlapAll" true))

(event `WeaponDeactive`
  (`PrimitiveComponent.SetCollisionEnabled` (`self.weponcollision`) "NoCollision"))

(fn `UserConstructionScript`)